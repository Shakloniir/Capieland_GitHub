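; BP_Pickup is a world item pickup that adds an item and amount to Kayra's inventory.
; The construction script takes mesh, scale and interact radius from the item class defaults.
; Sphere overlaps maintain Kayra's nearby-pickup queue, showing the first entry's label, or collect immediately if HasPickupCommand is set; mouse hover swaps material and cursor.
; Pickup records remaining amount by ID in LootedPickups, keeping partial leftovers and destroying emptied actors.
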(event `self.ReceiveBeginPlay`
  (`self.updateText`))

(event `onPickedUp`
  (params (kayraRef :type "/Game/CapieLand/Kayra/Blueprints/KayraBP Object Reference"))
  (bind _inventoryref (`/Game/CapieLand/Kayra/Blueprints/KayraBP.inventoryRef` kayraRef))
  (bind _inventoryref_2 (`/Game/CapieLand/Kayra/Blueprints/KayraBP.inventoryRef` kayraRef))
  (bind _nearbypickupactors (`/Game/CapieLand/Kayra/Blueprints/KayraBP.nearbyPickupActors` kayraRef))
  (bind _output (`|GetArrayItem` _nearbypickupactors))
  (`/Engine/EditorBlueprintResources/StandardMacros.IsValid` _inventoryref
    (:`Is Valid`
      (bind (_succes_ _rest) (`/Game/Inventory/InventorySystem/Bleprints/BP_Inventory.addItem` _inventoryref (`self.itemToAdd`) (`self.Amount`) true))
      (if _succes_
        (if (> _rest 0)
          (set `self.Amount` _rest)
          (`self.updateText`)
          (`KismetArrayLibrary.Array_Add` (`/Game/Inventory/InventorySystem/Bleprints/BP_Inventory.lootedPickups` _inventoryref_2) (make `/Game/Inventory/InventorySystem/Bleprints/Sturctures/S_SavedPickup` (`self.ID`) (`self.Amount`)))
          (else
            (`KismetArrayLibrary.Array_Add` (`/Game/Inventory/InventorySystem/Bleprints/BP_Inventory.lootedPickups` _inventoryref_2) (make `/Game/Inventory/InventorySystem/Bleprints/Sturctures/S_SavedPickup` (`self.ID`)))
            (`KismetArrayLibrary.Array_RemoveItem` _nearbypickupactors self)
            (`/Engine/EditorBlueprintResources/StandardMacros.IsValid` _output
              (:`Is Valid`
                (`SceneComponent.SetVisibility` (`/Game/Inventory/InventorySystem/Bleprints/ItemClasses/BP_Pickup.pickupText` _output) true false))
              (:`Is Not Valid`
                _))
            (if (`self.Hovered?`)
              (set `PlayerController.CurrentMouseCursor` "Default" (`GameplayStatics.GetPlayerController` 0))
              (`self.K2_DestroyActor`)
              (else
                (`self.K2_DestroyActor`)))))))))

(event `self.Sphere.OnComponentBeginOverlap`
  (params (OverlappedComponent :type "PrimitiveComponent Object Reference") (OtherActor :type "Actor Object Reference") (OtherComp :type "PrimitiveComponent Object Reference") (OtherBodyIndex :type Integer) (bFromSweep :type Boolean) (SweepResult :type "HitResult Structure (by ref)"))
  (bind _askayra_bp (cast `/Game/CapieLand/Kayra/Blueprints/KayraBP` OtherActor))
  (if (`self.hasPickupCommand?`)
    (`self.onPickedUp` _askayra_bp)
    (else
      (bind _nearbypickupactors (`/Game/CapieLand/Kayra/Blueprints/KayraBP.nearbyPickupActors` _askayra_bp))
      (if (> (`KismetArrayLibrary.Array_Length` _nearbypickupactors) 0)
        (`KismetArrayLibrary.Array_Add` _nearbypickupactors self)
        (else
          (`SceneComponent.SetVisibility` (`self.pickupText`) true false)
          (`KismetArrayLibrary.Array_Add` _nearbypickupactors self)
          (set `self.isInRange?` true))))))

(event `self.Sphere.OnComponentEndOverlap`
  (params (OverlappedComponent :type "PrimitiveComponent Object Reference") (OtherActor :type "Actor Object Reference") (OtherComp :type "PrimitiveComponent Object Reference") (OtherBodyIndex :type Integer))
  (bind _askayra_bp (cast `/Game/CapieLand/Kayra/Blueprints/KayraBP` OtherActor))
  (set `self.isInRange?` false)
  (bind _nearbypickupactors (`/Game/CapieLand/Kayra/Blueprints/KayraBP.nearbyPickupActors` _askayra_bp))
  (bind _output (`|GetArrayItem` _nearbypickupactors))
  (if (and (`KismetSystemLibrary.IsValid` _output) (== _output self))
    (`SceneComponent.SetVisibility` (`self.pickupText`) false false)
    (`KismetArrayLibrary.Array_RemoveItem` _nearbypickupactors self)
    (bind _output_2 (`|GetArrayItem` (`/Game/CapieLand/Kayra/Blueprints/KayraBP.nearbyPickupActors` _askayra_bp)))
    (`/Engine/EditorBlueprintResources/StandardMacros.IsValid` _output_2
      (:`Is Valid`
        (`SceneComponent.SetVisibility` (`/Game/Inventory/InventorySystem/Bleprints/ItemClasses/BP_Pickup.pickupText` _output_2) true false)))
    (else
      (`KismetArrayLibrary.Array_RemoveItem` _nearbypickupactors self))))

(event `self.staticMesh.OnBeginCursorOver`
  (params (TouchedComponent :type "PrimitiveComponent Object Reference"))
  (`self.onHovered`))

(event `self.staticMesh.OnEndCursorOver`
  (params (TouchedComponent :type "PrimitiveComponent Object Reference"))
  (`self.onUnhovered`))

(fn `onHovered`
  (set `PlayerController.CurrentMouseCursor` "Hand" (`GameplayStatics.GetPlayerController` 0))
  (set `self.Hovered?` true)
  (`PrimitiveComponent.SetMaterial` (`self.staticMesh`) 0 "/Game/Inventory/InventorySystem/Materials/hoveredPickupMat.hoveredPickupMat")
  (`SceneComponent.SetVisibility` (`self.pickupText`) true false)
  (return))

(fn `onUnhovered`
  (set `self.Hovered?` false)
  (set `PlayerController.CurrentMouseCursor` "Default" (`GameplayStatics.GetPlayerController` 0))
  (`PrimitiveComponent.SetMaterial` (`self.staticMesh`) 0 (`self.originalMat`))
  (`SceneComponent.SetVisibility` (`self.pickupText`) (`self.isInRange?`) false)
  (return))

(fn `updateText`
  (bind _aspickup_text (cast `/Game/Inventory/InventorySystem/Widgets/pickupText` (`WidgetComponent.GetUserWidgetObject` (`self.pickupText`)))
    (:`then`
      (`TextBlock.SetText` (`/Game/Inventory/InventorySystem/Widgets/pickupText.nameText` _aspickup_text) (`|FormatText` "{Name} ({Amount})" (`.Name_4_2FB29C944525261E7E90C5A20009D939` (break `/Game/Inventory/InventorySystem/Bleprints/Sturctures/S_ItemInfo` (defaults `Object` (`self.itemToAdd`)))) (`self.Amount`))))
    (:`CastFailed`
      _))
  (return))

(fn `UserConstructionScript`
  (bind _itemtoadd (`self.itemToAdd`))
  (bind _staticmesh (`self.staticMesh`))
  (bind (_name _description _icon _canbeused_ _usetext _canbestacked_ _category _internalname _weight _recipe _value _pickupmesh _meshscale _interactradius) (break `/Game/Inventory/InventorySystem/Bleprints/Sturctures/S_ItemInfo` (defaults `Object` _itemtoadd)))
  (if (`KismetSystemLibrary.IsValidClass` _itemtoadd)
    (`StaticMeshComponent.SetStaticMesh` _staticmesh _pickupmesh)
    (set `self.originalMat` (`PrimitiveComponent.GetMaterial` _staticmesh 0))
    (`SceneComponent.SetRelativeScale3D` _staticmesh _meshscale)
    (`SphereComponent.SetSphereRadius` (`self.Sphere`) _interactradius false)))