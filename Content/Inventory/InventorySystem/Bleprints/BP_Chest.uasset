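; BP_Chest is an interactable container that opens a slot-based storage screen for the Kayra player character.
; An overlap range toggles the prompt text and registers the chest as the player's NearbyChest.
; Interacting lazily spawns and reuses a BP_Storage actor, shows it with the inventory and stops player movement.
; A DoOnce blocks reopening until closing the storage hides it, restores walking and resets the gate.
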(event `onStorageClosed`
  (bind _kayraref (`self.kayraRef`))
  (bind _kayraref_2 (`self.kayraRef`))
  (bind _storageactor (`self.storageActor`))
  (bind _inventoryref (`/Game/CapieLand/Kayra/Blueprints/KayraBP.inventoryRef` _kayraref))
  (bind _inventoryref_2 (`/Game/CapieLand/Kayra/Blueprints/KayraBP.inventoryRef` _kayraref_2))
  (bind _charactermovement (`Character.CharacterMovement` _kayraref_2))
  (`/Game/Inventory/InventorySystem/Bleprints/BP_Storage.hideStorage` (`self.storageActor`))
  (`CharacterMovementComponent.SetMovementMode` (`Character.CharacterMovement` _kayraref) "MOVE_Walking" 0)
  (if (`/Game/Inventory/InventorySystem/Bleprints/BP_Inventory.isVisible?` _inventoryref)
    (`/Game/Inventory/InventorySystem/Bleprints/BP_Inventory.hideInventory` _inventoryref)
    (`/Game/Inventory/InventorySystem/Bleprints/BP_Inventory.showInventory` _inventoryref)
    (goto _label :!via `Reset`)
    (else
      (goto _label :!via `Reset`))))

(event `onInteract`
  (params (kayraRef :type "/Game/CapieLand/Kayra/Blueprints/KayraBP Object Reference"))
  (bind _kayraref (`self.kayraRef`))
  (bind _storageactor (`self.storageActor`))
  (bind _inventoryref (`/Game/CapieLand/Kayra/Blueprints/KayraBP.inventoryRef` _kayraref))
  (bind _charactermovement (`Character.CharacterMovement` _kayraref))
  (`/Engine/EditorBlueprintResources/StandardMacros.DoOnce` false :!label _label
    (:`Completed`
      (set `self.kayraRef` kayraRef)
      (`/Engine/EditorBlueprintResources/StandardMacros.IsValid` (`self.storageActor`)
        (:`Is Valid`
          _)
        (:`Is Not Valid`
          (bind _returnvalue (`|SpawnActorFromClass` "/Game/Inventory/InventorySystem/Bleprints/BP_Storage.BP_Storage_C" (`KismetMathLibrary.MakeTransform` (0.0 0.0 0.0)) "AlwaysSpawn" "OverrideRootScale" null (`self.amountOfSlots`) (`self.kayraRef`) (`self.slotsPerRow`) self null))
          (set `self.storageActor` _returnvalue)))
      (`/Game/Inventory/InventorySystem/Widgets/storageWidget.generateSlotWidgets` (`/Game/Inventory/InventorySystem/Bleprints/BP_Storage.storageWidget` _storageactor) _storageactor)
      (`/Game/Inventory/InventorySystem/Bleprints/BP_Storage.showStorage` _storageactor)
      (`/Game/Inventory/InventorySystem/Bleprints/BP_Inventory.hideInventory` _inventoryref)
      (`/Game/Inventory/InventorySystem/Bleprints/BP_Inventory.showInventory` _inventoryref)
      (`CharacterMovementComponent.DisableMovement` _charactermovement)
      (`MovementComponent.StopMovementImmediately` _charactermovement))))

(event `self.interactionRange.OnComponentBeginOverlap`
  (params (OverlappedComponent :type "PrimitiveComponent Object Reference") (OtherActor :type "Actor Object Reference") (OtherComp :type "PrimitiveComponent Object Reference") (OtherBodyIndex :type Integer) (bFromSweep :type Boolean) (SweepResult :type "HitResult Structure (by ref)"))
  (bind _askayra_bp (cast `/Game/CapieLand/Kayra/Blueprints/KayraBP` OtherActor))
  (`SceneComponent.SetVisibility` (`self.chestText`) true false)
  (set `/Game/CapieLand/Kayra/Blueprints/KayraBP.nearbyChest` self _askayra_bp))

(event `self.interactionRange.OnComponentEndOverlap`
  (params (OverlappedComponent :type "PrimitiveComponent Object Reference") (OtherActor :type "Actor Object Reference") (OtherComp :type "PrimitiveComponent Object Reference") (OtherBodyIndex :type Integer))
  (bind _askayra_bp (cast `/Game/CapieLand/Kayra/Blueprints/KayraBP` OtherActor))
  (`SceneComponent.SetVisibility` (`self.chestText`) false false)
  (set `/Game/CapieLand/Kayra/Blueprints/KayraBP.nearbyChest` null _askayra_bp))

(fn `UserConstructionScript`)