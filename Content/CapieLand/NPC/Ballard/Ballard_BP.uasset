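; Ballard NPC in CapieLand who gives a side quest, in Turkish dialogue, to find equipment dropped while fleeing Troldolar.
; Inherited conversation events chain the lines by index, with each finished line queuing the next.
; A timed decision lets the player ask about the problem or decline.
; Near the end of the quest explanation, it calls YanGörev1 on the player's Kaplan_BP, then ends the conversation after the last line.
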(event `self.OnDialogueEnd`
  (params (Index :type Integer))
  ;[1 1 1] On Dialogue End
  (switch `int` Index
    (:`0`
      (`self.AddCustomImportantDialogue` 1 (make `/Game/DialogueSystem/Blueprints/Structures/s_DialogueInfo` null "Eğer ordudan atılırsam anneme kim bakacak?" (`self.Name`))))
    (:`1`
      (`self.AddDecision` 0 (make `/Game/DialogueSystem/Blueprints/Structures/s_DecisionInfo` (make `/Game/DialogueSystem/Blueprints/Structures/s_DialogueInfo` null "Troldolardan nefret ediyorum." (`self.Name`)) (`|MakeArray` (make `/Game/DialogueSystem/Blueprints/Structures/s_OptionInfo` "Sorun Nedir?" "/Game/RadarSystem/Textures/Icon_SideQuest.Icon_SideQuest" "NewEnumerator1") (make `/Game/DialogueSystem/Blueprints/Structures/s_OptionInfo` "Meşgulüm") :!type "/Game/DialogueSystem/Blueprints/Structures/s_OptionInfo Structure") true)))
    (:`2`
      (`self.AddCustomImportantDialogue` 3 (make `/Game/DialogueSystem/Blueprints/Structures/s_DialogueInfo` null "Kuzey tarafında ağaçların arasından geçerken düşmüş olmalı" (`self.Name`) true)))
    (:`3`
      (`self.AddCustomImportantDialogue` 4 (make `/Game/DialogueSystem/Blueprints/Structures/s_DialogueInfo` null "Yerini bende tam olarak bilmiyorum" (`self.Name`))))
    (:`4`
      (`self.AddCustomImportantDialogue` 5 (make `/Game/DialogueSystem/Blueprints/Structures/s_DialogueInfo` null "Eğer bulup getitirsen sana karşılığını vereceğim" (`self.Name`)))
      (bind _askaplan_bp (cast `/Game/CapieLand/Kayra/Blueprints/Kaplan_BP` (`GameplayStatics.GetPlayerCharacter` 0)))
      (`/Game/CapieLand/Kayra/Blueprints/Kaplan_BP.Yan görev 1` _askaplan_bp))
    (:`5`
      (`self.EndConversation`))))

(event `self.AfterConversationSetup`
  ;[1 1 1] Adds the first dialogue
  (`self.AddCustomImportantDialogue` 0 (make `/Game/DialogueSystem/Blueprints/Structures/s_DialogueInfo` null "Lütfen bana yardım et!" (`self.Name`))))

(event `self.OnDecisionMade`
  (params (DecisionIndex :type Integer) (ChosenOptionIndex :type Integer))
  ;[1 1 1] On Decision Made
  (switch `int` DecisionIndex
    (:`0`
      (switch `int` ChosenOptionIndex
        (:`1`
          (`self.AddCustomImportantDialogue` 2 (make `/Game/DialogueSystem/Blueprints/Structures/s_DialogueInfo` null "Troldolardan kaçarken ekipmanımı düşürdüm" (`self.Name`))))
        (:`2`
          (`self.EndConversation`))))))

(fn `UserConstructionScript`
  (`parent.UserConstructionScript`))