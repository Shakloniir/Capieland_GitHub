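; Troldo enemy character that takes melee hits from Kayra, the player, and strikes back with a hitbox attached to its skull socket.
; Incoming overlaps pick damage by component name, then trigger material flash, sound, knockback, a brief attack interruption and death at zero health.
; Anim-notify-named events toggle the attack hitbox, which damages and launches the player unless the shield blocks it.
; A timeline fades the name and health bar on proximity or hit.
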(event `self.Hasar alma Kapsülü.OnComponentBeginOverlap`
  (params (OverlappedComponent :type "PrimitiveComponent Object Reference") (OtherActor :type "Actor Object Reference") (OtherComp :type "PrimitiveComponent Object Reference") (OtherBodyIndex :type Integer) (bFromSweep :type Boolean) (SweepResult :type "HitResult Structure (by ref)"))
  (bind _enemy_widget (`self.Enemy Widget`))
  (bind _capsulecomponent (`self.CapsuleComponent`))
  (bind _currenthealth (`self.CurrentHealth`))
  (bind _healthbar (`/Game/Enemy/EnemyWidget.HealthBar` _enemy_widget))
  (bind _nametext (`/Game/Enemy/EnemyWidget.NameText` _enemy_widget))
  ;[1 0.1611 0.1198] Hasar ve Vuruş hissi
  (if (not (`self.Dead?`))
    (bind _askayra_bp (cast `/Game/CapieLand/Kayra/Blueprints/KayraBP` (`GameplayStatics.GetPlayerCharacter` 0)))
    (if (not (`self.Is Launched?`))
      (switch `string` (`KismetSystemLibrary.GetObjectName` OtherComp)
        (:`Alan Etkili Hasar`
          (set `self.CurrentHealth` (`KismetMathLibrary.Clamp` (- (`self.CurrentHealth`) (`/Game/CapieLand/Kayra/Blueprints/KayraBP.Alan Etkili Damage` _askayra_bp)) 0 30)))
        (:`Odaklı Hasar`
          (set `self.CurrentHealth` (`KismetMathLibrary.Clamp` (- (`self.CurrentHealth`) (`/Game/CapieLand/Kayra/Blueprints/KayraBP.Odaklı Damage` _askayra_bp)) 0 30)))
        (:`Kalkan Saldırısı`
          (set `self.CurrentHealth` (`KismetMathLibrary.Clamp` (- (`self.CurrentHealth`) (`/Game/CapieLand/Kayra/Blueprints/KayraBP.ShieldDamage` _askayra_bp)) 0 30))))
      (`|ExecutionSequence`
        (:`then_0`
          (`PrimitiveComponent.SetMaterial` (`self.Mesh`) 7 "/Game/Enemy/Hasar.Hasar")
          (`KismetSystemLibrary.Delay` 0.1)
          (`PrimitiveComponent.SetMaterial` (`self.Mesh`) 7 null)
          (bind (_returnvalue_x _returnvalue_y) (`KismetMathLibrary.BreakVector` (`KismetMathLibrary.GetForwardVector` (`KismetMathLibrary.FindLookAtRotation` (`SceneComponent.K2_GetComponentLocation` OverlappedComponent) (`SceneComponent.K2_GetComponentLocation` (`/Game/CapieLand/Kayra/Blueprints/KayraBP.Kılıcın Ucu` _askayra_bp))))))
          (bind _returnvalue (+ (* (`KismetMathLibrary.MakeVector` _returnvalue_x _returnvalue_y) -700.0) (0.0 0.0 200.0)))
          (`GameplayStatics.PlaySoundAtLocation` "/Game/CapieLand/SoundEffect/BaseballDrop_BW_47655.BaseballDrop_BW_47655" _returnvalue (struct) 1.0 1.0 0.0 null null null))
        (:`then_1`
          (`self.LaunchCharacter` _returnvalue true true)
          (`KismetSystemLibrary.LineTraceSingle` (0.0 0.0 0.0) (0.0 0.0 0.0) "TraceTypeQuery1")
          (set `self.Is Launched?` true)
          (`KismetSystemLibrary.Delay` 0.2)
          (set `self.Is Launched?` false)
          (`KismetSystemLibrary.PrintString` (`KismetStringLibrary.Conv_IntToString` _currenthealth))
          (if (<= _currenthealth 0)
            (set `self.Attacking Player` false)
            (set `self.Attack1` false)
            (set `self.Dead?` true)
            (set `self.Moving?` false)
            (`SkeletalMeshComponent.PlayAnimation` (`self.Mesh`) "/Game/Enemy/Troldo/Animation/troldo_animations_1_4_Anim_rig_death1.troldo_animations_1_4_Anim_rig_death1" false)
            (`PrimitiveComponent.SetCollisionResponseToChannel` _capsulecomponent "ECC_Pawn" "ECR_Ignore")
            (`PrimitiveComponent.SetCollisionResponseToChannel` _capsulecomponent "ECC_Visibility" "ECR_Ignore")
            (`KismetSystemLibrary.Delay` 3.0)
            (`self.K2_DestroyActor`)))
        (:`then_2`
          (`PrimitiveComponent.SetMaterial` (`self.Mesh`) 0 "/Game/Enemy/Hasar.Hasar")
          (`KismetSystemLibrary.Delay` 0.1)
          (`PrimitiveComponent.SetMaterial` (`self.Mesh`) 0 null))
        (:`then_3`
          (set `self.Attack1` false)
          (`KismetSystemLibrary.Delay` 0.2)
          (set `self.Attack1` true))
        (:`then_4`
          ;;[1 1 1] Can barı
          (set `self.Enemy Widget` (cast `/Game/Enemy/EnemyWidget` (`WidgetComponent.GetUserWidgetObject` (`self.Health Bar`)) :!pure true) :!label _label)
          (`ProgressBar.SetPercent` _healthbar (/ (`KismetMathLibrary.Conv_IntToDouble` (`self.CurrentHealth`)) 30.0))
          (`TextBlock.SetText` _nametext "Troldo")
          (bind (_direction `_i_sim_ve_can_opaklığı`) (`Timeline|Bar görünürlüğü Setleme` :!label _label_2)
            (:`Update`
              (`Widget.SetRenderOpacity` _healthbar `_i_sim_ve_can_opaklığı`)
              (`TextBlock.SetOpacity` _nametext `_i_sim_ve_can_opaklığı`))))))))

(event `self.İsim ve Can Gösterme Alanı.OnComponentBeginOverlap`
  (params (OverlappedComponent :type "PrimitiveComponent Object Reference") (OtherActor :type "Actor Object Reference") (OtherComp :type "PrimitiveComponent Object Reference") (OtherBodyIndex :type Integer) (bFromSweep :type Boolean) (SweepResult :type "HitResult Structure (by ref)"))
  ;[1 0.1611 0.1198] Hasar ve Vuruş hissi
  ;;[1 1 1] Can barı
  (if (== OtherActor (`self.Player referans`))
    (goto _label)))

(event `self.İsim ve Can Gösterme Alanı.OnComponentEndOverlap`
  (params (OverlappedComponent :type "PrimitiveComponent Object Reference") (OtherActor :type "Actor Object Reference") (OtherComp :type "PrimitiveComponent Object Reference") (OtherBodyIndex :type Integer))
  ;[1 0.1611 0.1198] Hasar ve Vuruş hissi
  ;;[1 1 1] Can barı
  (if (== OtherActor (`self.Player referans`))
    (goto _label_2 :!via `Reverse`)))

(event `self.Troldo Saldırısı.OnComponentBeginOverlap`
  (params (OverlappedComponent :type "PrimitiveComponent Object Reference") (OtherActor :type "Actor Object Reference") (OtherComp :type "PrimitiveComponent Object Reference") (OtherBodyIndex :type Integer) (bFromSweep :type Boolean) (SweepResult :type "HitResult Structure (by ref)"))
  ;[1 1 1] KARAKTERE HASAR VER
  (`/Engine/EditorBlueprintResources/StandardMacros.IsValid` OtherActor
    (:`Is Valid`
      (bind _askayra_bp (cast `/Game/CapieLand/Kayra/Blueprints/KayraBP` (`GameplayStatics.GetPlayerCharacter` 0)))
      (if (`KismetStringLibrary.EqualEqual_StrStr` (`KismetSystemLibrary.GetObjectName` OtherComp) "Kalkan Savunması")
        (`PrimitiveComponent.SetCollisionEnabled` (`self.Troldo Saldırısı`) "NoCollision")
        (`|ExecutionSequence`
          (:`then_0`
            (set `self.Vurabilir mi?` false)
            (`KismetSystemLibrary.Delay` 0.15)
            (set `self.Vurabilir mi?` true))
          (:`then_1`
            (`/Game/CapieLand/Kayra/Blueprints/KayraBP.Kalkan_Geri_Tepmesi` _askayra_bp)))
        (else
          (`KismetSystemLibrary.Delay` 0.01)
          (if (`self.Vurabilir mi?`)
            (set `/Game/CapieLand/Kayra/Blueprints/KayraBP.Health` (- (`/Game/CapieLand/Kayra/Blueprints/KayraBP.Health` _askayra_bp) (`self.Hasar`)) _askayra_bp)
            (`PrimitiveComponent.SetCollisionEnabled` (`self.Troldo Saldırısı`) "NoCollision")
            (bind (_returnvalue_x _returnvalue_y) (`KismetMathLibrary.BreakVector` (`KismetMathLibrary.GetForwardVector` (`KismetMathLibrary.FindLookAtRotation` (`self.K2_GetActorLocation`) (`SceneComponent.K2_GetComponentLocation` (`Actor.RootComponent` _askayra_bp))))))
            (bind (_returnvalue_x_2 _returnvalue_y_2) (`KismetMathLibrary.BreakVector` (* (`KismetMathLibrary.MakeVector` _returnvalue_x _returnvalue_y) 600.0)))
            (`self.LaunchCharacter` _askayra_bp (`KismetMathLibrary.MakeVector` _returnvalue_x_2 _returnvalue_y_2 100.0) true true)))))))

(event `Saldır başlangıç`
  ;[1 1 1] ANİM NOTİFY
  (if (`self.Attack1`)
    (`PrimitiveComponent.SetCollisionEnabled` (`self.Troldo Saldırısı`) "QueryOnly")))

(event `Saldırı bitiş`
  ;[1 1 1] ANİM NOTİFY
  (`PrimitiveComponent.SetCollisionEnabled` (`self.Troldo Saldırısı`) "NoCollision"))

(event `self.ReceiveBeginPlay`
  ;[1 1 1] Event Begin Play
  (bind _askayra_bp (cast `/Game/CapieLand/Kayra/Blueprints/KayraBP` (`GameplayStatics.GetPlayerCharacter` 0)))
  (set `self.Player referans` _askayra_bp))

(event `Attack`
  (`SkeletalMeshComponent.PlayAnimation` (`self.Mesh`) "/Game/Enemy/Troldo/Animation/troldo_animations_1_4_Anim_rig_hit1.troldo_animations_1_4_Anim_rig_hit1" false))

(fn `Can Barı`)

(fn `UserConstructionScript`
  (`SceneComponent.K2_AttachToComponent` (`self.Troldo Saldırısı`) (`self.Mesh`) "kafatas" "KeepWorld" "KeepWorld" "KeepWorld" true))